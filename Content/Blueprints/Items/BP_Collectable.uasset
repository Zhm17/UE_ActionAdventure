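; BP_Collectable is a coin pickup that spins in place and vanishes when the player collects it.
; BeginPlay picks a random spin direction, and Tick rotates the static mesh about yaw by that fixed per-frame amount.
; On sphere overlap, it checks that the other actor's instigator is BP_MainCharacter, then calls AddCoins on MainGameMode and destroys itself.
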(event `self.ReceiveBeginPlay`
  ;[0.9362 0 1] Animation
  (set `self.RotationSpeed` (`KismetMathLibrary.SelectFloat` 1.5 -1.5 (`KismetMathLibrary.RandomBool`))))

(event `self.ReceiveTick`
  (params (DeltaSeconds :type "Float (single-precision)"))
  ;[0.9362 0 1] Animation
  (`SceneComponent.K2_AddRelativeRotation` (`self.StaticMesh`) (`KismetMathLibrary.MakeRotator` 0.0 0.0 (`self.RotationSpeed`)) false false))

(event `self.SphereCollisionComponent.OnComponentBeginOverlap`
  (params (OverlappedComponent :type "PrimitiveComponent Object Reference") (OtherActor :type "Actor Object Reference") (OtherComp :type "PrimitiveComponent Object Reference") (OtherBodyIndex :type Integer) (bFromSweep :type Boolean) (SweepResult :type "HitResult Structure (by ref)"))
  ;[1 0 0] Collision
  (cast `/Game/Blueprints/BP_MainCharacter` (`self.GetInstigator` OtherActor))
  ;[0 1 0.08176] Update Coins Counter
  (bind _asmain_game_mode (cast `/Game/Blueprints/MainGameMode` (`GameplayStatics.GetGameMode`)))
  (`/Game/Blueprints/MainGameMode.AddCoins` _asmain_game_mode)
  (`self.K2_DestroyActor`))

(fn `UserConstructionScript`)