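; MainGameMode is a game mode that tracks coin collection and puts the coin HUD on screen.
; BeginPlay creates the WBP_CoinsDisplay widget, stores it as HeadsUpDisplay and adds it to the viewport.
; AddCoins increments CoinsCollected, calls CountCoinsRemaining and returns the new total.
; CountCoinsRemaining sets and returns CoinsRemaining by counting all BP_Collectable actors in the world, rather than decrementing a counter.
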(event `self.ReceiveBeginPlay`
  ;[0.303 0 1] HUDs
  (bind _returnvalue (`|CreateWidget` "/Game/Blueprints/UI/WBP_CoinsDisplay.WBP_CoinsDisplay_C"))
  (bind _output_get (set `self.HeadsUpDisplay` _returnvalue))
  (`UserWidget.AddToViewport` _output_get 0))

(fn `AddCoins`
  (returns (CoinsCollected :type Integer))
  (bind _result (`/Engine/EditorBlueprintResources/StandardMacros.IncrementInt` (`self.CoinsCollected`))
    (:`  `
      (bind _output_get (set `self.CoinsCollected` _result))
      (`self.CountCoinsRemaining`)
      (return _output_get))))

(fn `CountCoinsRemaining`
  (returns (CoinsRemaining :type Integer))
  (bind _outactors (`GameplayStatics.GetAllActorsOfClass` "/Game/Blueprints/Items/BP_Collectable.BP_Collectable_C"))
  (bind _output_get (set `self.CoinsRemaining` (`KismetArrayLibrary.Array_Length` _outactors)))
  (return _output_get))

(fn `UserConstructionScript`)