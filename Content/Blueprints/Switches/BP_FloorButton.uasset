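; BP_FloorButton is a pressure switch that opens a door while BP_MainCharacter stands on it.
; Its sphere collision starts disabled at BeginPlay and turns on through the OnEnableCollision event.
; Overlap lowers the button mesh and calls OnOpenDoor; leaving waits SecondsPressed, then raises it and calls OnCloseDoor.
; The door is found with GetActorOfClass, so it targets whichever BP_Door that returns rather than an assigned reference.
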(event `self.ReceiveBeginPlay`
  (`PrimitiveComponent.SetCollisionEnabled` (`self.SphereCollision`) "NoCollision"))

(event `OnEnableCollision`
  (`PrimitiveComponent.SetCollisionEnabled` (`self.SphereCollision`) "QueryAndPhysics"))

(event `self.SphereCollision.OnComponentBeginOverlap`
  (params (OverlappedComponent :type "PrimitiveComponent Object Reference") (OtherActor :type "Actor Object Reference") (OtherComp :type "PrimitiveComponent Object Reference") (OtherBodyIndex :type Integer) (bFromSweep :type Boolean) (SweepResult :type "HitResult Structure (by ref)"))
  ;[1 0 0] Collision
  (cast `/Game/Blueprints/BP_MainCharacter` OtherActor)
  ;[0 1 0.09172] On Pressed
  (set `self.Pressed` true)
  (`self.Button ZMovement` -20.0)
  ;[0.9663 0 1] Open / Close Door
  (bind _returnvalue (`GameplayStatics.GetActorOfClass` "/Game/Blueprints/Door/BP_Door.BP_Door_C"))
  (`/Game/Blueprints/Door/BP_Door.OnOpenDoor` _returnvalue))

(event `self.SphereCollision.OnComponentEndOverlap`
  (params (OverlappedComponent :type "PrimitiveComponent Object Reference") (OtherActor :type "Actor Object Reference") (OtherComp :type "PrimitiveComponent Object Reference") (OtherBodyIndex :type Integer))
  ;[1 0 0] Collision
  (cast `/Game/Blueprints/BP_MainCharacter` OtherActor)
  ;[0 1 0.09172] On Pressed
  (`KismetSystemLibrary.Delay` (`self.SecondsPressed`))
  (set `self.Pressed` false)
  (`self.Button ZMovement` 0.0)
  ;[0.9663 0 1] Open / Close Door
  (bind _returnvalue (`GameplayStatics.GetActorOfClass` "/Game/Blueprints/Door/BP_Door.BP_Door_C"))
  (`/Game/Blueprints/Door/BP_Door.OnCloseDoor` _returnvalue))

(fn `Button ZMovement`
  (params (ZRelativeValue :type "Float (double-precision)"))
  (bind _button_staticmesh (`self.Button_StaticMesh`))
  (bind (_relativelocation_x _relativelocation_y) (`KismetMathLibrary.BreakVector` (`SceneComponent.RelativeLocation` _button_staticmesh)))
  (`SceneComponent.K2_SetRelativeLocation` _button_staticmesh (`KismetMathLibrary.MakeVector` _relativelocation_x _relativelocation_y ZRelativeValue) false false))

(fn `UserConstructionScript`)